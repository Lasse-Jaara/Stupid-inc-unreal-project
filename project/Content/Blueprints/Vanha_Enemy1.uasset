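; Enemy pawn, apparently an older version by its name, that either shoots at the player or wanders on the navmesh.
; BeginPlay forces IsSeeingPlayer true, zeroes PawnSensing's peripheral vision angle and calls GunFire once.
; GunFire stops movement and spawns a Bullet at Aiming's relative transform if IsPlayerHidden is true.
; When not seeing the player, it calls MoveRandomly to pick a nearby navigable point.
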(event `GunFire`
  ; Gunning
  (if (`self.isSeeingPlayer?`)
    (`MovementComponent.StopMovementImmediately` (`self.CharacterMovement`))
    (if (`self.isPlayerHidden?`)
      (`|SpawnActorFromClass` "/Game/Blueprints/Bullet.Bullet_C" (`SceneComponent.GetRelativeTransform` (`self.aiming`)) "Undefined" "MultiplyWithRoot" null null))
    (else
      (`self.MoveRandomly` (0.0 0.0 0.0)))))

(event `self.ReceiveBeginPlay`
  ; Movement
  (set `self.isSeeingPlayer?` true)
  (`PawnSensingComponent.SetPeripheralVisionAngle` (`self.PawnSensing`) 0.0)
  (`self.GunFire`))

(fn `MoveRandomly`
  (params (Origin :type "Vector Structure (by ref)"))
  (bind _randomlocation (`NavigationSystemV1.K2_GetRandomLocationInNavigableRadius` Origin 500.0 null "/Script/AIModule.NavFilter_AIControllerDefault"))
  (`AIBlueprintHelperLibrary.SimpleMoveToLocation` null _randomlocation))

(fn `UserConstructionScript`)